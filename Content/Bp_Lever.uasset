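; Bp_Lever is a one-use lever that the hero can pull by releasing F while inside its box trigger.
; Box overlaps with Bp_Hero enable and disable player input on the lever.
; The F handler checks LeverUsed and a DoOnce before calling Activate, which plays the SwitchRotation timeline to rotate the Lever.
; When the timeline finishes, it sets LeverUsed and prints that state.
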(event `Activate`
  (bind (_direction _newtrack_0) (`Timeline|SwitchRotation` :!via `PlayFromStart`)
    (:`Update`
      (`SceneComponent.K2_SetRelativeRotation` (`self.Lever`) (`KismetMathLibrary.MakeRotator` (.x _newtrack_0) (.y _newtrack_0) (.z _newtrack_0)) false false))
    (:`Finished`
      (bind _output_get (set `self.LeverUsed` true))
      (`KismetSystemLibrary.PrintString` (`KismetStringLibrary.Concat_StrStr` "LeverUsed" (`KismetStringLibrary.Conv_BoolToString` _output_get))))))

(event `self.Box.OnComponentBeginOverlap`
  (params (OverlappedComponent :type "PrimitiveComponent Object Reference") (OtherActor :type "Actor Object Reference") (OtherComp :type "PrimitiveComponent Object Reference") (OtherBodyIndex :type Integer) (bFromSweep :type Boolean) (SweepResult :type "HitResult Structure (by ref)"))
  (cast `/Game/Bp_Hero` OtherActor)
  (`self.EnableInput` (`GameplayStatics.GetPlayerController` 0)))

(event `self.Box.OnComponentEndOverlap`
  (params (OverlappedComponent :type "PrimitiveComponent Object Reference") (OtherActor :type "Actor Object Reference") (OtherComp :type "PrimitiveComponent Object Reference") (OtherBodyIndex :type Integer))
  (cast `/Game/Bp_Hero` OtherActor)
  (`self.DisableInput` (`GameplayStatics.GetPlayerController` 0)))

(event `Key|F`
  (params (Key :type "Key Structure"))
  (:`Released`
    (if (not (`self.LeverUsed`))
      (`/Engine/EditorBlueprintResources/StandardMacros.DoOnce` false
        (:`Completed`
          (`self.Activate`))))))

(fn `UserConstructionScript`)