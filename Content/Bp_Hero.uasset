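; Hero Blueprint that handles the player's combat input: blocking, directional melee attacks and spell casting.
; Block and Attack set state booleans, with attack direction taken from movement axes and a DoOnce re-armed on release.
; AttackTrace toggles overlap events on the Box hitbox, which applies damage and spawns a HitSpark on overlapping other actors.
; Middle mouse spawns BP_Spell at the Arrow1 transform.
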(event `InputAction|Block`
  (params (Key :type "Key Structure"))
  ;[1 1 1] Set Blocking boolean
  (:`Pressed`
    (set `self.Blocking?` true))
  (:`Released`
    (set `self.Blocking?` false)))

(event `InputAction|Attack`
  (params (Key :type "Key Structure"))
  ;[1 1 1] AttackingAnim
  (:`Pressed`
    (`/Engine/EditorBlueprintResources/StandardMacros.DoOnce` false :!label _label
      (:`Completed`
        (set `self.Attacking?` true)
        (if (== (`self.GetInputAxisValue`) 0.0)
          _
          (elif (< (`self.GetInputAxisValue`) 0.0)
            (set `self.AttackLeft` true)
            (else
              (set `self.AttackRight` true))))
        (if (< (`self.GetInputAxisValue`) 0.0)
          (set `self.AttackBackward` true)
          (else
            (set `self.AttackForward` true))))))
  (:`Released`
    (set `self.Attacking?` false)
    (set `self.AttackForward` false)
    (set `self.AttackBackward` false)
    (set `self.AttackLeft` false)
    (set `self.AttackRight` false)
    (goto _label :!via `Reset`)))

(event `self.Box.OnComponentBeginOverlap`
  (params (OverlappedComponent :type "PrimitiveComponent Object Reference") (OtherActor :type "Actor Object Reference") (OtherComp :type "PrimitiveComponent Object Reference") (OtherBodyIndex :type Integer) (bFromSweep :type Boolean) (SweepResult :type "HitResult Structure (by ref)"))
  ;[1 1 1] AttackingAnim
  (if (not (== OtherActor self))
    (`GameplayStatics.ApplyDamage` OtherActor 1.0)
    (`|SpawnActorFromClass` "/Game/HitSpark.HitSpark_C" (`KismetMathLibrary.MakeTransform` (`SceneComponent.K2_GetComponentLocation` OverlappedComponent)) "Undefined" "OverrideRootScale" null null)))

(event `Key|MiddleMouseButton`
  (params (Key :type "Key Structure"))
  (:`Pressed`
    (`|SpawnActorFromClass` "/Game/BP_Spell.BP_Spell_C" (`SceneComponent.K2_GetComponentToWorld` (`self.Arrow1`)) "AdjustIfPossibleButAlwaysSpawn" "OverrideRootScale" null "NewEnumerator1" null)))

(fn `AttackTrace`
  (params (Condition :type Boolean))
  (bind _box (`self.Box`))
  (if Condition
    (set `PrimitiveComponent.bGenerateOverlapEvents` true _box)
    (else
      (`/Engine/EditorBlueprintResources/StandardMacros.IsValid` _box
        (:`Is Valid`
          (set `PrimitiveComponent.bGenerateOverlapEvents` false _box))))))

(fn `UserConstructionScript`
  (`parent.UserConstructionScript`))