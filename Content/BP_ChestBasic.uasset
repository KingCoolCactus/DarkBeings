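; BP_ChestBasic is a chest that the hero opens to spawn an item.
; A Box overlap with Bp_Hero toggles player input on the chest, so the Interact action only works nearby.
; Releasing Interact calls Open, which runs once through a DoOnce and plays a timeline rotating the Lid on roll.
; When the timeline finishes, it spawns ItemToSpawn at the Arrow component's transform.
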(event `Open`
  (`/Engine/EditorBlueprintResources/StandardMacros.DoOnce` false
    (:`Completed`
      (bind (_direction _newtrack_2) (`Timeline|Opening` :!via `PlayFromStart`)
        (:`Update`
          (bind _result (`/Engine/EditorBlueprintResources/StandardMacros.NegateFloat` (.x _newtrack_2))
            (:`  `
              (`SceneComponent.K2_SetRelativeRotation` (`self.Lid`) (`KismetMathLibrary.MakeRotator` _result) false false))))
        (:`Finished`
          (`|SpawnActorFromClass` (`self.Item To Spawn`) (`SceneComponent.K2_GetComponentToWorld` (`self.Arrow`)) "Undefined" "OverrideRootScale" null null))))))

(event `self.Box.OnComponentBeginOverlap`
  (params (OverlappedComponent :type "PrimitiveComponent Object Reference") (OtherActor :type "Actor Object Reference") (OtherComp :type "PrimitiveComponent Object Reference") (OtherBodyIndex :type Integer) (bFromSweep :type Boolean) (SweepResult :type "HitResult Structure (by ref)"))
  (cast `/Game/Bp_Hero` OtherActor)
  (`self.EnableInput` (`GameplayStatics.GetPlayerController` 0)))

(event `self.Box.OnComponentEndOverlap`
  (params (OverlappedComponent :type "PrimitiveComponent Object Reference") (OtherActor :type "Actor Object Reference") (OtherComp :type "PrimitiveComponent Object Reference") (OtherBodyIndex :type Integer))
  (cast `/Game/Bp_Hero` OtherActor)
  (`self.DisableInput` (`GameplayStatics.GetPlayerController` 0)))

(event `InputAction|Interact`
  (params (Key :type "Key Structure"))
  (:`Released`
    (`self.Open`)))

(fn `UserConstructionScript`)