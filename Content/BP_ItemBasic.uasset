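; BP_ItemBasic is a spinning pickup item that fully restores the hero's health.
; Two seconds after BeginPlay it enables overlap events on its Capsule, while Tick slowly rotates the Mesh.
; When a Bp_Hero overlaps the Capsule, the item sets PlayerHealth to PlayerMaxHealth and destroys itself.
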(event `self.ReceiveBeginPlay`
  (`KismetSystemLibrary.Delay` 2.0)
  (set `PrimitiveComponent.bGenerateOverlapEvents` true (`self.Capsule`)))

(event `self.ReceiveTick`
  (params (DeltaSeconds :type "Float (single-precision)"))
  (`SceneComponent.K2_AddLocalRotation` (`self.Mesh`) (struct :`Yaw` 0.1) false false))

(event `self.Capsule.OnComponentBeginOverlap`
  (params (OverlappedComponent :type "PrimitiveComponent Object Reference") (OtherActor :type "Actor Object Reference") (OtherComp :type "PrimitiveComponent Object Reference") (OtherBodyIndex :type Integer) (bFromSweep :type Boolean) (SweepResult :type "HitResult Structure (by ref)"))
  (bind _asbp_hero (cast `/Game/Bp_Hero` OtherActor))
  (set `/Game/AFPC/Blueprints/AFPCharacter/Character/AFPCharacter_Default.PlayerHealth` (`/Game/AFPC/Blueprints/AFPCharacter/Character/AFPCharacter_Default.PlayerMaxHealth` _asbp_hero) _asbp_hero)
  (`self.K2_DestroyActor`))

(fn `UserConstructionScript`)