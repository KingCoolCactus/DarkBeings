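; BP_DoorBasic is an interactable door that slides vertically between its starting height and a fixed raised position.
; Overlap with Bp_Hero enables player input, end overlap from any actor disables it, and releasing Interact calls Trigger.
; Unless Locked, Trigger plays the DoorMove timeline forward or in reverse, lerping the door's Z.
; On finish it flips Open and, with AutoClose set, re-triggers after a delay to close.
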(event `self.ReceiveBeginPlay`
  (bind (_returnvalue_x _returnvalue_y _returnvalue_z) (`KismetMathLibrary.BreakVector` (`SceneComponent.K2_GetComponentLocation` (`self.Door`))))
  (bind _output_get (set `self.StartingZ` _returnvalue_z))
  (set `self.TargetZ` (+ _output_get 205.0)))

(event `Trigger`
  (bind (_returnvalue_x _returnvalue_y _returnvalue_z) (`KismetMathLibrary.BreakVector` (`SceneComponent.K2_GetComponentLocation` (`self.Door`))))
  (if (`self.Locked?`)
    _
    (elif (`self.Open?`)
      (bind (_direction _alpha) (`Timeline|DoorMove` :!via `ReverseFromEnd` :!label _label)
        (:`Update`
          (`SceneComponent.K2_SetWorldLocation` (`self.Door`) (`KismetMathLibrary.MakeVector` _returnvalue_x _returnvalue_y (`KismetMathLibrary.Lerp` (`self.StartingZ`) (`self.TargetZ`) _alpha)) false false))
        (:`Finished`
          (if (`self.Open?`)
            (set `self.Open?` false)
            (else
              (set `self.Open?` true)
              ;[1 1 1] AutoClose
              (if (`self.AutoClose`)
                (`KismetSystemLibrary.Delay` (`self.AutoCloseTimer`))
                (`self.Trigger`))))))
      (else
        (goto _label :!via `PlayFromStart`)))))

(event `self.Box.OnComponentBeginOverlap`
  (params (OverlappedComponent :type "PrimitiveComponent Object Reference") (OtherActor :type "Actor Object Reference") (OtherComp :type "PrimitiveComponent Object Reference") (OtherBodyIndex :type Integer) (bFromSweep :type Boolean) (SweepResult :type "HitResult Structure (by ref)"))
  (cast `/Game/Blueprints/PlayerChar/Bp_Hero` OtherActor)
  (`self.EnableInput` (`GameplayStatics.GetPlayerController` 0))
  (`KismetSystemLibrary.PrintString` "Door In Range"))

(event `self.Box.OnComponentEndOverlap`
  (params (OverlappedComponent :type "PrimitiveComponent Object Reference") (OtherActor :type "Actor Object Reference") (OtherComp :type "PrimitiveComponent Object Reference") (OtherBodyIndex :type Integer))
  (`self.DisableInput` (`GameplayStatics.GetPlayerController` 0))
  (`KismetSystemLibrary.PrintString` "Door OUT of Range"))

(event `InputAction|Interact`
  (params (Key :type "Key Structure"))
  (:`Released`
    (`self.Trigger`)))

(fn `UserConstructionScript`)