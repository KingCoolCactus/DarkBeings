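; BP_Spell is a player magic actor that deals damage on contact and removes itself after a set lifetime.
; On BeginPlay it activates its particle system after a short delay and schedules its own destruction after LifeSpan.
; When its Sphere begins an overlap, it applies damage and spawns a HitSpark effect at the sphere's transform, without destroying itself.
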(event `self.ReceiveBeginPlay`
  (`|ExecutionSequence`
    (:`then_0`
      (`KismetSystemLibrary.Delay` 0.2)
      (`ActorComponent.Activate` (`self.ParticleSystem`) false))
    (:`then_1`
      (`KismetSystemLibrary.Delay` (`self.LifeSpan`))
      (`self.K2_DestroyActor`))))

(event `self.Sphere.OnComponentBeginOverlap`
  (params (OverlappedComponent :type "PrimitiveComponent Object Reference") (OtherActor :type "Actor Object Reference") (OtherComp :type "PrimitiveComponent Object Reference") (OtherBodyIndex :type Integer) (bFromSweep :type Boolean) (SweepResult :type "HitResult Structure (by ref)"))
  (`GameplayStatics.ApplyDamage` null 1.0)
  (`|SpawnActorFromClass` "/Game/Blueprints/PlayerChar/HitSpark.HitSpark_C" (`SceneComponent.K2_GetComponentToWorld` (`self.Sphere`)) "Undefined" "OverrideRootScale" null null))

(fn `UserConstructionScript`)