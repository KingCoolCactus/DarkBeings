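; BP_NB_MasterItemOLD is an item pickup actor that shows a collection widget when the player touches it.
; When the player character overlaps PickupSphere, it creates UI_NB_ItemCollect using the name, icon and stack count from BPNBItemComponent.
; It adds the widget to the viewport, then destroys itself after a very short delay.
; The graph itself makes no inventory update.
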(event `self.PickupSphere.OnComponentBeginOverlap`
  (params (OverlappedComponent :type "PrimitiveComponent Object Reference") (OtherActor :type "Actor Object Reference") (OtherComp :type "PrimitiveComponent Object Reference") (OtherBodyIndex :type Integer) (bFromSweep :type Boolean) (SweepResult :type "HitResult Structure (by ref)"))
  (bind _bp_nb_itemcomponent (`self.BP_NB_ItemComponent`))
  (if (== OtherActor (`GameplayStatics.GetPlayerCharacter` 0))
    (bind _returnvalue (`|CreateWidget` "/Game/Blueprints/Inventory/UI_NB_ItemCollect.UI_NB_ItemCollect_C" null (`/Game/Blueprints/Inventory/BP_NB_ItemComponent.ItemName` _bp_nb_itemcomponent) (`/Game/Blueprints/Inventory/BP_NB_ItemComponent.Icon` _bp_nb_itemcomponent) (`/Game/Blueprints/Inventory/BP_NB_ItemComponent.NumberInStack` _bp_nb_itemcomponent)))
    (`UserWidget.AddToViewport` _returnvalue 0)
    (`KismetSystemLibrary.Delay` 0.01)
    (`self.K2_DestroyActor`)))

(fn `UserConstructionScript`)