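; BP_TargetBarrel is a damageable barrel target that can drop an item when destroyed.
; Any damage prints a hurt message and reduces its Health.
; At zero health or below it optionally spawns a configured item class at its Arrow component's transform, gated by SpawnItem, then destroys itself.
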(event `self.ReceiveAnyDamage`
  (params (Damage :type "Float (single-precision)") (DamageType :type "DamageType Object Reference") (InstigatedBy :type "Controller Object Reference") (DamageCauser :type "Actor Object Reference"))
  (`KismetSystemLibrary.PrintString` "OWWW That Hurt" true true (struct :`R` 1.0 :`B` 0.019891 :`A` 1.0))
  (bind _output_get (set `self.Health` (- (`self.Health`) Damage)))
  (if (<= _output_get 0.0)
    (if (`self.SpawnItem?`)
      (`|SpawnActorFromClass` (`self.ITEMTOSPAWN`) (`SceneComponent.K2_GetComponentToWorld` (`self.Arrow`)) "Undefined" "OverrideRootScale" null null))
    (`self.K2_DestroyActor`)))

(fn `UserConstructionScript`)