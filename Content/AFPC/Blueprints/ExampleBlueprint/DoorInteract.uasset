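; Interactable door Blueprint that moves a door vertically while its Button component receives an activated Interaction event.
; The Gate timeline lerps the door between two heights, using a hold or release curve chosen by the Release flag.
; A looping timer treats the player moving out of range like deactivation, which reverses the timeline unless Release or Complete is set.
; Timeline completion sets Complete, which blocks further play or reversal.
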(event `/Game/AFPC/Blueprints/AFPCharacter/Interfaces/PlayerInterface.Interaction`
  (params (`Activation?` :type Boolean) (ActorSender :type "Actor Object Reference") (HitComponent :type "PrimitiveComponent Object Reference"))
  (bind _door (`self.Door`))
  (if `Activation?`
    (if (== HitComponent (`self.Button`))
      (bind _returnvalue (`KismetSystemLibrary.K2_SetTimerDelegate` (delegate `Player_CheckDistance`) 0.1 true))
      (set `self.Timer_CheckPlayerDistance` _returnvalue)
      (if (not (`self.Complete`))
        (bind (_direction _doorlerphold _doorlerprelease) (`Timeline|Gate` :!label _label)
          (:`Update`
            (if (`self.Release`)
              (`SceneComponent.K2_SetRelativeLocation` _door (`KismetMathLibrary.VLerp` (0.0 -50.0 -151.0) (0.0 -50.0 150.0) _doorlerprelease) false false)
              (else
                (`SceneComponent.K2_SetRelativeLocation` _door (`KismetMathLibrary.VLerp` (0.0 -50.0 150.0) (0.0 -50.0 -151.0) _doorlerphold) false false)
                (`/Engine/EditorBlueprintResources/StandardMacros.DoOnce` false :!label _label_2
                  (:`Completed`
                    (set `self.Complete` false))))))
          (:`Finished`
            (set `self.Complete` true)
            (set `self.Release` false)
            (goto _label_2 :!via `Reset`)))))
    (else
      (if (not (`self.Complete`)) :!label _label_3
        (`KismetSystemLibrary.K2_ClearAndInvalidateTimerHandle` (`self.Timer_CheckPlayerDistance`))
        (if (not (`self.Release`))
          (goto _label :!via `Reverse`))))))

(event `Player_CheckDistance`
  (if (> (`self.GetDistanceTo` (`GameplayStatics.GetPlayerCharacter` 0)) 300.0)
    (`KismetSystemLibrary.K2_ClearAndInvalidateTimerHandle` (`self.Timer_CheckPlayerDistance`))
    (goto _label_3)))

(fn `UserConstructionScript`)