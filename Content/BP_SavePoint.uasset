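; BP_SavePoint is a save point actor that Bp_Hero lights up by interacting nearby; the graph contains no save logic.
; Its spotlights and particle system are deactivated on BeginPlay.
; Sphere overlap enables and disables the actor's input for player 0, gating the Interact action to that range.
; Releasing Interact calls Activate through a DoOnce that is never reset, switching the effects on a single time.
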(event `self.ReceiveBeginPlay`
  (`ActorComponent.Deactivate` (`self.SpotLight`))
  (`ActorComponent.Deactivate` (`self.ParticleSystem`))
  (`ActorComponent.Deactivate` (`self.SpotLight`)))

(event `Activate`
  (`ActorComponent.Activate` (`self.SpotLight`) false)
  (`ActorComponent.Activate` (`self.ParticleSystem`) false)
  (`ActorComponent.Activate` (`self.SpotLight`) false))

(event `self.Sphere.OnComponentBeginOverlap`
  (params (OverlappedComponent :type "PrimitiveComponent Object Reference") (OtherActor :type "Actor Object Reference") (OtherComp :type "PrimitiveComponent Object Reference") (OtherBodyIndex :type Integer) (bFromSweep :type Boolean) (SweepResult :type "HitResult Structure (by ref)"))
  (cast `/Game/Bp_Hero` OtherActor)
  (`self.EnableInput` (`GameplayStatics.GetPlayerController` 0)))

(event `self.Sphere.OnComponentEndOverlap`
  (params (OverlappedComponent :type "PrimitiveComponent Object Reference") (OtherActor :type "Actor Object Reference") (OtherComp :type "PrimitiveComponent Object Reference") (OtherBodyIndex :type Integer))
  (cast `/Game/Bp_Hero` OtherActor)
  (`self.DisableInput` (`GameplayStatics.GetPlayerController` 0)))

(event `InputAction|Interact`
  (params (Key :type "Key Structure"))
  (:`Released`
    (`/Engine/EditorBlueprintResources/StandardMacros.DoOnce` false
      (:`Completed`
        (`self.Activate`)))))

(fn `UserConstructionScript`)